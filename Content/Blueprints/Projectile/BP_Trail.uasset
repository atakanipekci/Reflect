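; BP_Trail is an actor in the Projectile folder that carries a Niagara trail effect driven by external events.
; Its events move it to a given location without sweeping, activate the Niagara component, and destroy it after a given delay.
; A stored start scale normalizes later scale values into the Niagara ScaleMultiplier variable, skipped when the start scale is not positive.
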(event `SetLocation`
  (params (Location :type "Vector Structure"))
  (`self.K2_SetActorLocation` Location))

(event `SetStartScale`
  (params (StartScale :type "Float (double-precision)"))
  (set `self.StartScale` StartScale))

(event `SetScale`
  (params (Scale :type "Float (double-precision)"))
  (bind _startscale (`self.StartScale`))
  (if (> _startscale 0.0)
    (`NiagaraComponent.SetVariableFloat` (`self.NiagaraComponent`) "ScaleMultiplier" (/ Scale _startscale))))

(event `DestroyWithDelay`
  (params (Delay :type "Float (double-precision)"))
  (`KismetSystemLibrary.Delay` Delay)
  (`self.K2_DestroyActor`))

(event `ActivateNiagara`
  (`ActorComponent.Activate` (`self.NiagaraComponent`) false))

(fn `UserConstructionScript`)