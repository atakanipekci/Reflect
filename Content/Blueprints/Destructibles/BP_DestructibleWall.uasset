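; BP_DestructibleWall is a destructible wall that shatters at a hit location when its Explode event is called.
; DestroyGeometry enables Geometry Collection physics, then applies Chaos fields: radial strain using the damage threshold and Sphere radius, plus radial velocity, both raw and culled by that falloff.
; If the CollisionBox is valid, Explode removes it and destroys the actor after DestroyTime.
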(event `self.ReceiveBeginPlay`)

(event `self.Explode`
  (params (HitAt :type "Vector Structure (by ref)"))
  (bind _collisionbox (`self.CollisionBox`))
  (`self.DestroyGeometry` HitAt)
  (`/Engine/EditorBlueprintResources/StandardMacros.IsValid` _collisionbox
    (:`Is Valid`
      (`ActorComponent.K2_DestroyComponent` _collisionbox)
      (`KismetSystemLibrary.Delay` (`self.DestroyTime`))
      (`self.K2_DestroyActor`))))

(fn `DestroyGeometry`
  (params (HitAt :type "Vector Structure"))
  (locals (HitLocation :type "Vector Structure"))
  (bind _returnvalue (`RadialVector.SetRadialVector` (`self.RadialVector`) 1000.0 (`local.HitLocation`)))
  (bind _returnvalue_2 (`RadialFalloff.SetRadialFalloff` (`self.RadialFalloff`) (`|GetArrayItem` (`GeometryCollectionComponent.DamageThreshold` (`self.GeometryCollection`))) 0.0 1.0 0.0 (`SphereComponent.SphereRadius` (`self.Sphere`)) (`local.HitLocation`) "Field_FallOff_None"))
  (set `local.HitLocation` HitAt)
  (`PrimitiveComponent.SetSimulatePhysics` (`self.GeometryCollection`) true)
  (`FieldSystemComponent.ApplyPhysicsField` (`self.FieldSystem`) true "Field_ExternalClusterStrain" null _returnvalue_2)
  (`FieldSystemComponent.ApplyPhysicsField` (`self.FieldSystem`) true "Field_LinearVelocity" null _returnvalue)
  (`FieldSystemComponent.ApplyPhysicsField` (`self.FieldSystem`) true "Field_LinearVelocity" null (`CullingField.SetCullingField` (`self.CullingField`) _returnvalue_2 _returnvalue "Field_Culling_Outside")))

(fn `UserConstructionScript`)