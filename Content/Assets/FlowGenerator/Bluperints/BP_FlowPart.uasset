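; Flow cable actor that animates a material effect along a spline and, on activation, tries to trigger an attached actor after a play-rate-based delay.
; Construction builds spline mesh segments from the spline points.
; A timeline moves a plane and optional particle trail along the spline, feeding plane position and normal to segment materials, or to placed static meshes in FlowStaticMesh mode.
; It re-sets the previous segment at its endpoint to absorb framerate and speed gaps.
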(event `self.ReceiveBeginPlay`
  (bind _p_trail_trace (`self.P_Trail_Trace`))
  (if (not (`self.FlowStaticMesh`))
    (for _array_element (`self.SplineMesh`)
      (`MeshComponent.SetVectorParameterValueOnMaterials` _array_element "normal" (0.0 0.0 0.0))))
  (set `self.TotalStepCount` (- (`SplineComponent.GetNumberOfSplinePoints` (`self.Spline`)) 1))
  (for _index (range (+ (`self.TotalStepCount`) 1))
    (`KismetArrayLibrary.Array_Add` (`self.SplinePointDistance`) (`SplineComponent.GetDistanceAlongSplineAtSplinePoint` (`self.Spline`) _index)))
  (if (`self.SpawnParticle`)
    (`SceneComponent.SetVisibility` _p_trail_trace false false)
    (else
      (`ActorComponent.K2_DestroyComponent` _p_trail_trace)))
  ;[1 1 1] Reinit if flow static mesh
  (if (`self.FlowStaticMesh`)
    (for _array_element_2 (`self.StaticMeshes`)
      (`MeshComponent.SetVectorParameterValueOnMaterials` (`StaticMeshActor.StaticMeshComponent` _array_element_2) "normal" (0.0 0.0 0.0)))))

(event `LaunchSequence`
  (params (PlayRate :type "Float (double-precision)" :default 1.0))
  (if (`self.SpawnParticle`)
    (`SceneComponent.SetVisibility` (`self.P_Trail_Trace`) true false))
  (`TimelineComponent.SetPlayRate` (`self.Timeline_0`) PlayRate)
  (bind (_direction _newtrack_0) (`Timeline|Timeline_0` :!via `PlayFromStart` :!label _label)
    (:`Update`
      (`self.UpdatePlaneAlongSpline` _newtrack_0)
      (set `self.Distance` _newtrack_0)
      (if (`self.FlowStaticMesh`)
        (`self.SendPosToStaticMesh`)
        (else
          (`self.ManageCurrentStep` (`self.Distance`))
          (`self.UpdateSplineMat`))))
    (:`Finished`
      (if (`self.SpawnParticle`)
        (`SceneComponent.SetVisibility` (`self.P_Trail_Trace`) false false)))))

(event `PlayPause`
  (params (PLayRate :type "Float (double-precision)" :default 1.0))
  (`TimelineComponent.SetPlayRate` (`self.Timeline_0`) PLayRate)
  (`/Engine/EditorBlueprintResources/StandardMacros.FlipFlop`
    (:`A`
      (goto _label))
    (:`B`
      (goto _label :!via `Stop`))))

(event `Reset`
  (bind (_returnvalue_location _returnvalue_rotation) (`KismetMathLibrary.BreakTransform` (`SceneComponent.K2_GetComponentToWorld` (`self.DefaultSceneRoot`))))
  ;[1 1 1] Reset from beginning
  (set `self.CurrentStep` 0)
  (`SceneComponent.K2_SetWorldTransform` (`self.Plane`) (`KismetMathLibrary.MakeTransform` _returnvalue_location _returnvalue_rotation (0.2 0.2 0.2)) false false)
  (`self.ResetAllMat`))

(event `self.ActivateCable`
  (params (bActivate :type Boolean))
  (if bActivate
    (`self.LaunchSequence` (`self.PlayRate`))
    (`KismetSystemLibrary.Delay` (/ 1.0 (`self.PlayRate`)))
    (if (`self.bIsActive`)
      (`self.TryActivatingAttachedActor`))
    (else
      (`self.Reset`))))

(fn `BuildSpline`
  (bind _spline (`self.Spline`))
  (bind _splinescale (`self.SplineScale`))
  (`KismetArrayLibrary.Array_Clear` (`self.SplineMesh`))
  (for _index (range (+ (- (`SplineComponent.GetNumberOfSplinePoints` (`self.Spline`)) 2) 1))
    (bind _returnvalue (`AddComponent|NODE_AddSplineMeshComponent-0`))
    (`KismetArrayLibrary.Array_AddUnique` (`self.SplineMesh`) _returnvalue)
    (`StaticMeshComponent.SetStaticMesh` _returnvalue (`self.StaticMesh`))
    (`PrimitiveComponent.SetMaterial` _returnvalue 0 (`self.Mat`))
    (`SplineMeshComponent.SetForwardAxis` _returnvalue (`self.ForwardAxis`) true)
    (`SceneComponent.K2_AttachToComponent` _returnvalue (`self.Spline`) "None" "KeepRelative" "KeepRelative" "KeepRelative" true)
    (bind _returnvalue_2 (+ _index 1))
    (`SplineMeshComponent.SetStartAndEnd` _returnvalue (`SplineComponent.GetLocationAtSplinePoint` _spline _index "Local") (`SplineComponent.GetTangentAtSplinePoint` _spline _index "Local") (`SplineComponent.GetLocationAtSplinePoint` _spline _returnvalue_2 "Local") (`SplineComponent.GetTangentAtSplinePoint` _spline _returnvalue_2 "Local") true)
    (`SplineMeshComponent.SetEndScale` _returnvalue _splinescale true)
    (`SplineMeshComponent.SetStartScale` _returnvalue _splinescale true)
    (`PrimitiveComponent.SetCastShadow` _returnvalue (`self.CastShadow`))))

(fn `ManageCurrentStep`
  (params (DistanceFactor :type "Float (double-precision)"))
  (bind _spline (`self.Spline`))
  (bind _output (`|GetArrayItem` (`self.SplinePointDistance`) (`self.CurrentStep`)))
  (bind _returnvalue (/ (* DistanceFactor (`SplineComponent.GetDistanceAlongSplineAtSplinePoint` _spline (- (`SplineComponent.GetNumberOfSplinePoints` _spline) 1))) 1.0))
  (if (`KismetMathLibrary.InRange_FloatFloat` _returnvalue _output (`|GetArrayItem` (`self.SplinePointDistance`) (+ (`self.CurrentStep`) 1)))
    (set `self.CurrentStep` (+ (`self.CurrentStep`) 1))
    (elif (<= _output _returnvalue)
      (set `self.CurrentStep` (- (`self.CurrentStep`) 1)))))

(fn `ResetAllMat`
  (if (not (`self.FlowStaticMesh`))
    (for _array_element (`self.SplineMesh`)
      (`MeshComponent.SetVectorParameterValueOnMaterials` _array_element "pos" (0.0 0.0 0.0))
      (`MeshComponent.SetVectorParameterValueOnMaterials` _array_element "normal" (0.0 0.0 0.0)))))

(fn `SendPosToStaticMesh`
  (for _array_element (`self.StaticMeshes`)
    (bind _staticmeshcomponent (`StaticMeshActor.StaticMeshComponent` _array_element))
    (`MeshComponent.SetVectorParameterValueOnMaterials` _staticmeshcomponent "pos" (`SceneComponent.K2_GetComponentLocation` (`self.Plane`)))
    (`MeshComponent.SetVectorParameterValueOnMaterials` _staticmeshcomponent "normal" (`SceneComponent.GetForwardVector` (`self.Plane`)))))

(fn `UpdatePlaneAlongSpline`
  (params (DistanceFactor :type "Float (double-precision)"))
  (bind _spline (`self.Spline`))
  (bind _spline_2 (`self.Spline`))
  (bind _returnvalue (+ (/ (* DistanceFactor (`SplineComponent.GetDistanceAlongSplineAtSplinePoint` _spline (- (`SplineComponent.GetNumberOfSplinePoints` _spline) 1))) 1.0) (`self.SpeedAdjustment`)))
  (bind _returnvalue_2 (`SplineComponent.GetLocationAtDistanceAlongSpline` _spline_2 _returnvalue "World"))
  (`SceneComponent.K2_SetWorldLocationAndRotation` (`self.Plane`) _returnvalue_2 (`SplineComponent.GetRotationAtDistanceAlongSpline` _spline_2 _returnvalue "World") false false)
  (if (`self.SpawnParticle`)
    (`SceneComponent.K2_SetWorldLocation` (`self.P_Trail_Trace`) _returnvalue_2 false false)))

(fn `UpdateSplineMat`
  (bind _speedadjustment (`self.SpeedAdjustment`))
  (bind _spline (`self.Spline`))
  (bind _output (`|GetArrayItem` (`self.SplineMesh`)))
  (bind _returnvalue (`KismetMathLibrary.Clamp` (- (`self.CurrentStep`) 1) 0 (`self.TotalStepCount`)))
  (bind _returnvalue_2 (`SplineComponent.GetDirectionAtSplinePoint` _spline _returnvalue "World"))
  (bind _output_2 (`|GetArrayItem` (`self.SplineMesh`) (`KismetMathLibrary.Clamp` (- (`self.CurrentStep`) 2) 0 (`self.TotalStepCount`))))
  (bind _output_3 (`|GetArrayItem` (`self.SplineMesh`) (`KismetMathLibrary.Clamp` (- (`self.CurrentStep`) 1) 0 (`self.TotalStepCount`))))
  (if (> (`self.TotalStepCount`) 1)
    (`MeshComponent.SetVectorParameterValueOnMaterials` _output_3 "pos" (`SceneComponent.K2_GetComponentLocation` (`self.Plane`)))
    (`MeshComponent.SetVectorParameterValueOnMaterials` _output_3 "normal" (`SceneComponent.GetForwardVector` (`self.Plane`)))
    ;[1 1 1] Force the last spline mesh update (prevent fps and speed issues)
    (if (>= (`self.CurrentStep`) 2)
      (`MeshComponent.SetVectorParameterValueOnMaterials` _output_2 "pos" (+ (`SplineComponent.GetLocationAtSplinePoint` _spline _returnvalue "World") (* _returnvalue_2 (`KismetMathLibrary.MakeVector` _speedadjustment _speedadjustment _speedadjustment))))
      (`MeshComponent.SetVectorParameterValueOnMaterials` _output_2 "normal" _returnvalue_2))
    (else
      (`MeshComponent.SetVectorParameterValueOnMaterials` _output "pos" (`SceneComponent.K2_GetComponentLocation` (`self.Plane`)))
      (`MeshComponent.SetVectorParameterValueOnMaterials` _output "normal" (`SceneComponent.GetForwardVector` (`self.Plane`))))))

(fn `UpdateSplineMesh`
  (bind _spline (`self.Spline`))
  ;[1 1 1] Not called in this BP but usefull if the spline is edited at runtime
  (for (_array_element _array_index) (`self.SplineMesh`)
    (bind _returnvalue (+ _array_index 1))
    (`SplineMeshComponent.SetStartAndEnd` _array_element (`SplineComponent.GetLocationAtSplinePoint` _spline _array_index "Local") (`SplineComponent.GetTangentAtSplinePoint` _spline _array_index "Local") (`SplineComponent.GetLocationAtSplinePoint` _spline _returnvalue "Local") (`SplineComponent.GetTangentAtSplinePoint` _spline _returnvalue "Local") true)))

(fn `UserConstructionScript`
  (`/Engine/EditorBlueprintResources/StandardMacros.IsValid` (`self.StaticMesh`)
    (:`Is Valid`
      (`self.BuildSpline`))
    (:`Is Not Valid`
      _))
  (if (not (`self.SpawnParticle`))
    (`SceneComponent.SetVisibility` (`self.P_Trail_Trace`) false false))
  (if (`self.FlowStaticMesh`)
    (for _array_element (`self.StaticMeshes`)
      (bind _staticmeshcomponent (`StaticMeshActor.StaticMeshComponent` _array_element))
      (`MeshComponent.SetVectorParameterValueOnMaterials` _staticmeshcomponent "normal" (1.0 0.0 0.0))
      (`MeshComponent.SetVectorParameterValueOnMaterials` _staticmeshcomponent "pos" (`SceneComponent.K2_GetComponentLocation` _staticmeshcomponent)))))